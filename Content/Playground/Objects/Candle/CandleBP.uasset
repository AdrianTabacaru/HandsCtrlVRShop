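; CandleBP is a grabbable candle with a fixed hand grip that lights when a Flame actor touches its wick sphere.
; Lighting happens once, spawning a new Flame attached to the sphere, with a timeline driving its intensity.
; On every second overlap of its collision box, it destroys itself and spawns a replacement just above the CandleCubeBase of the first ProduseCat_1_BP found at BeginPlay.
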(event `self.ReceiveBeginPlay`
  (bind _returnvalue (`KismetMathLibrary.MakeTransform` (2.1 0.2 9.7) (struct :`Pitch` 73.0 :`Yaw` 111.0 :`Roll` 178.0)))
  ;[0 1 0.2318] Begin Play
  (`|ExecutionSequence`
    (:`then_0`
      (add `PrimitiveComponent.OnComponentBeginOverlap` (`self.Sphere`) (delegate `OnComponentBeginOverlap_Event_0`))
      (`/UVRF/Hands/Grabable.SetFixedGrab` (`self.Grabable`) (`self.Candle`) _returnvalue "/UVRF/Hands/Model/Animations/Grabs/grab_round_medium.grab_round_medium" _returnvalue))
    (:`then_1`
      (bind _outactors (`GameplayStatics.GetAllActorsOfClass` "/Game/Spawnable-ProduseCat_1/ProduseCat_1_BP.ProduseCat_1_BP_C")))))

(event `OnComponentBeginOverlap_Event_0`
  (params (OverlappedComponent :type "PrimitiveComponent Object Reference") (OtherActor :type "Actor Object Reference") (OtherComp :type "PrimitiveComponent Object Reference") (OtherBodyIndex :type Integer) (bFromSweep :type Boolean) (SweepResult :type "HitResult Structure (by ref)"))
  (if (not (`self.Lit`))
    (cast `/Game/Playground/Objects/Flame/Flame` OtherActor)
    (set `self.Lit` true)
    (bind _returnvalue (`|SpawnActorFromClass` "/Game/Playground/Objects/Flame/Flame.Flame_C" (`KismetMathLibrary.MakeTransform` (0.0 0.0 0.0)) "Undefined" "OverrideRootScale" null null))
    (bind _output_get (set `self.FlameRef` _returnvalue))
    (`self.K2_AttachToComponent` _output_get (`self.Sphere`) "None" "SnapToTarget" "KeepWorld" "KeepRelative" true)
    (bind (_direction _intensity) (`Timeline|FlameStart`)
      (:`Update`
        (`/Game/Playground/Objects/Flame/Flame.SetIntensity` (`self.FlameRef`) _intensity)))))

(event `self.BoxCollisionCandle.OnComponentBeginOverlap`
  (params (OverlappedComponent :type "PrimitiveComponent Object Reference") (OtherActor :type "Actor Object Reference") (OtherComp :type "PrimitiveComponent Object Reference") (OtherBodyIndex :type Integer) (bFromSweep :type Boolean) (SweepResult :type "HitResult Structure (by ref)"))
  (`/Engine/EditorBlueprintResources/StandardMacros.FlipFlop`
    (:`B`
      (`KismetSystemLibrary.PrintString` "Candle Box Collision")
      (`self.K2_DestroyActor`)
      (`/Engine/EditorBlueprintResources/StandardMacros.DoOnce` false
        (:`Completed`
          (bind (_returnvalue_x _returnvalue_y _returnvalue_z) (`KismetMathLibrary.BreakVector` (`SceneComponent.K2_GetComponentLocation` (`/Game/Spawnable-ProduseCat_1/ProduseCat_1_BP.CandleCubeBase` (`|GetArrayItem` (stale `self.ReceiveBeginPlay` _outactors))))))
          (`|SpawnActorFromClass` "CandleBP_C" (`KismetMathLibrary.MakeTransform` (`KismetMathLibrary.MakeVector` _returnvalue_x _returnvalue_y (+ _returnvalue_z 10.0)) (struct) (1.0 1.0 1.0)) "AdjustIfPossibleButAlwaysSpawn" "OverrideRootScale" null null))))))

(fn `UserConstructionScript`)