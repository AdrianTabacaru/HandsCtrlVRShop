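; Grabbable VR electric toothbrush product that toggles on with X in the left hand (haptics, sound, spinning head) or A in the right (haptics only).
; Tick tracks the grabbing hand, reveals three color cubes on roll tilt, and mutes LargeDisplay overlaps while a hand touches it.
; Cube overlaps recolor it through struct-driven dynamic materials.
; Every second overlap of its box respawns it at the product base, keeping the last color.
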(event `self.Periuta_v2_BODY.OnComponentBeginOverlap`
  (params (OverlappedComponent :type "PrimitiveComponent Object Reference") (OtherActor :type "Actor Object Reference") (OtherComp :type "PrimitiveComponent Object Reference") (OtherBodyIndex :type Integer) (bFromSweep :type Boolean) (SweepResult :type "HitResult Structure (by ref)"))
  ;[0 0.1742 1] To Remember
)

(event `self.Periuta_v2_BODY.OnComponentEndOverlap`
  (params (OverlappedComponent :type "PrimitiveComponent Object Reference") (OtherActor :type "Actor Object Reference") (OtherComp :type "PrimitiveComponent Object Reference") (OtherBodyIndex :type Integer))
  ;[0 0.1742 1] To Remember
)

(event `InputAction|PrintStringTestNow`
  (params (Key :type "Key Structure")))

(event `self.ReceiveTick`
  (params (DeltaSeconds :type "Float (single-precision)"))
  (bind _returnvalue (`GameplayStatics.GetPlayerController` 0))
  (bind _grabbedbymylefthand (`self.GrabbedByMyLeftHand`))
  (bind _cuberoz (`self.CubeRoz`))
  (bind _boxcollisioncheckwithhandcollisionsphere (`self.BoxCollisionCheckWithHandCollisionSphere`))
  (bind _grabable (`self.Grabable`))
  (bind _grabbedbymyrighthand (`self.GrabbedByMyRightHand`))
  (bind _periuta_v2_body (`self.Periuta_v2_BODY`))
  (bind _cubenegru (`self.CubeNegru`))
  (bind _cubealb (`self.CubeAlb`))
  (bind (_returnvalue_location _returnvalue_rotation) (`KismetMathLibrary.BreakTransform` (`SceneComponent.K2_GetComponentToWorld` _periuta_v2_body)))
  (bind _returnvalue_roll (`KismetMathLibrary.BreakRotator` (`SceneComponent.K2_GetComponentRotation` (`self.Periuta_v2_BODY`))))
  (bind _grabbed (`/UVRF/Hands/Grabable.IsGrabbed` _grabable))
  ;[1 0 0.5732] Tick
  (`|ExecutionSequence`
    (:`then_0`
      ;[1 1 1] Define Grabbing Hand, Start Haptics, Rotation and Sound
      (`|ExecutionSequence`
        (:`then_0`
          (`|ExecutionSequence`
            (:`then_0`
              (if (and (`self.LeftHandXClicked`) _grabbedbymylefthand)
                (`/Engine/EditorBlueprintResources/StandardMacros.DoOnce` false :!label _label
                  (:`Completed`
                    (`/Engine/EditorBlueprintResources/StandardMacros.FlipFlop`
                      (:`A`
                        (`|ExecutionSequence`
                          (:`then_0`
                            (`PlayerController.PlayHapticEffect` _returnvalue "/UVRF/Haptics/Periuta2.Periuta2" "Left" 4.0 true)
                            (`|ExecutionSequence`
                              (:`then_0`
                                (bind _returnvalue_2 (`GameplayStatics.SpawnSoundAttached` "/Game/Audio/ElectricBrush/ElectricBrush_Start_Cue.ElectricBrush_Start_Cue" _periuta_v2_body "None" _returnvalue_location _returnvalue_rotation "SnapToTargetIncludingScale" true 1.0 1.0 0.0 null null)))
                              (:`then_1`
                                (bind (_direction _newtrack_0) (`Timeline|HeadRotationLeftHand` :!label _label_2)
                                  (:`Update`
                                    (`SceneComponent.K2_SetRelativeRotation` (`self.Periuta_v2_HEAD`) (`KismetMathLibrary.MakeRotator` 0.0 _newtrack_0) false false))))
                              (:`then_2`
                                (set `self.IntForSoundStop` 1))
                              (:`then_3`
                                (switch `int` (`self.IntForSoundStop`) :!label _label_3
                                  (:`0`
                                    (set `self.MySoundIsPlaying` false))
                                  (:`1`
                                    (set `self.MySoundIsPlaying` true))))))))
                      (:`B`
                        (`|ExecutionSequence`
                          (:`then_0`
                            (`PlayerController.StopHapticEffect` _returnvalue "Left" :!label _label_4)
                            (`|ExecutionSequence`
                              (:`then_0`
                                (set `self.IntForSoundStop` 0))
                              (:`then_1`
                                (`KismetSystemLibrary.Delay` 0.4)
                                (goto _label_2 :!via `Stop`))
                              (:`then_2`
                                (`|ExecutionSequence`
                                  (:`then_0`
                                    (if (`self.MySoundIsPlaying`)
                                      (`AudioComponent.Stop` _returnvalue_2)
                                      (`GameplayStatics.SpawnSoundAttached` "/Game/Audio/ElectricBrush/ElectricBrush_Stop_Cue.ElectricBrush_Stop_Cue" _periuta_v2_body "None" _returnvalue_location _returnvalue_rotation "SnapToTargetIncludingScale" false 1.0 1.0 0.0 null null false)))))
                              (:`then_3`
                                (goto _label_3)))))))))
                (else
                  (goto _label :!via `Reset`))))
            (:`then_1`
              (if (not _grabbedbymylefthand)
                (`|ExecutionSequence`
                  (:`then_0`
                    (goto _label_4)))))))
        (:`then_1`
          (`|ExecutionSequence`
            (:`then_0`
              (if (and (`self.RightHandAClicked`) _grabbedbymyrighthand)
                (`/Engine/EditorBlueprintResources/StandardMacros.DoOnce` false :!label _label_5
                  (:`Completed`
                    (`/Engine/EditorBlueprintResources/StandardMacros.FlipFlop`
                      (:`A`
                        (`PlayerController.PlayHapticEffect` _returnvalue "/UVRF/Haptics/Periuta2.Periuta2" "Right" 4.0 true))
                      (:`B`
                        (`PlayerController.StopHapticEffect` _returnvalue "Right" :!label _label_6)))))
                (else
                  (goto _label_5 :!via `Reset`))))
            (:`then_1`
              (if (not _grabbedbymyrighthand)
                (goto _label_6)))))
        (:`then_3`
          ;;[1 1 1] Grabbed By Hand Type
          (if _grabbed
            (switch `EControllerHand` (`/UVRF/Hands/HandBP.HandType` (`/UVRF/Hands/Grabable.Hand` _grabable)) ; This Is The Key
              (:`Left`
                (if _grabbed
                  (set `self.GrabbedByMyLeftHand` true)
                  (set `self.GrabbedByMyRightHand` false :!label _label_7)
                  (else
                    (set `self.GrabbedByMyLeftHand` false :!label _label_8))))
              (:`Right`
                (if _grabbed
                  (set `self.GrabbedByMyRightHand` true)
                  (goto _label_8)
                  (else
                    (goto _label_7)))))))
        (:`then_4`
          (if (not _grabbed)
            (`|ExecutionSequence`
              (:`then_0`
                (goto _label_8))
              (:`then_1`
                (goto _label_7)))))))
    (:`then_1`
      ;[1 1 1] Tilt to choose color
      (if (`KismetMathLibrary.InRange_FloatFloat` _returnvalue_roll -70.0 -20.0)
        (`SceneComponent.SetVisibility` _cuberoz true false)
        (`SceneComponent.SetVisibility` _cubealb true false)
        (`SceneComponent.SetVisibility` _cubenegru true false)
        (set `PrimitiveComponent.bGenerateOverlapEvents` true _cuberoz)
        (set `PrimitiveComponent.bGenerateOverlapEvents` true _cubenegru)
        (set `PrimitiveComponent.bGenerateOverlapEvents` true _cubealb)
        (else
          (`SceneComponent.SetVisibility` _cuberoz false false)
          (`SceneComponent.SetVisibility` _cubealb false false)
          (`SceneComponent.SetVisibility` _cubenegru false false)
          (set `PrimitiveComponent.bGenerateOverlapEvents` false _cuberoz)
          (set `PrimitiveComponent.bGenerateOverlapEvents` false _cubenegru)
          (set `PrimitiveComponent.bGenerateOverlapEvents` false _cubealb))))
    (:`then_2`
      ;[1 1 1] Check Which Hand is overlapping (It checks the self Box Collision with VR Pawn Sphere Collision) - After it sets the INT
      (`|ExecutionSequence`
        (:`then_0`
          (bind _outactors (`GameplayStatics.GetAllActorsOfClass` "/UVRF/Pawn/VRPawn.VRPawn_C")))
        (:`then_1`
          (bind _output (`|GetArrayItem` _outactors))
          (bind _output_get (set `self.OverlappedByLeftHand` (`PrimitiveComponent.IsOverlappingComponent` _boxcollisioncheckwithhandcollisionsphere (`/UVRF/Pawn/VRPawn.SphereCollisionLeftHand` _output))))
          (if _output_get
            _))
        (:`then_2`
          (bind _output_get_2 (set `self.OverlappedByRightHand` (`PrimitiveComponent.IsOverlappingComponent` _boxcollisioncheckwithhandcollisionsphere (`/UVRF/Pawn/VRPawn.SphereCollisionRightHand` _output))))
          (if _output_get_2
            _))
        (:`then_3`
          ;[1 1 1] Disables Hand Lines Collision with Large Display BP
          (if (or (`self.OverlappedByLeftHand`) (`self.OverlappedByRightHand`))
            (bind _output_2 (`|GetArrayItem` (stale `self.ReceiveBeginPlay` _outactors_2)))
            (`/Game/VR_Table+Display/LargeDisplay_BP.SetLargeDisplayIntTo1` _output_2) ; 1 Ignores Overlap
            (else
              (`/Game/VR_Table+Display/LargeDisplay_BP.SetLargeDisplayIntTo0` _output_2) ; 0 Accepts Overlap
            )))))))

(event `self.ReceiveBeginPlay`
  ;[0 1 0.001442] Begin Play
  (`|ExecutionSequence`
    (:`then_0`
      ;[1 1 1] Grabbed object position and rotation
      (`/UVRF/Hands/Grabable.SetFixedGrab` (`self.Grabable`) (`self.Periuta_v2_BODY`) (`KismetMathLibrary.MakeTransform` (5.0 -5.0 10.0) (struct :`Pitch` -48.0 :`Yaw` 20.0 :`Roll` 102.0)) "/UVRF/Hands/Model/Animations/Grabs/grab_Periuta1.grab_Periuta1" (`KismetMathLibrary.MakeTransform` (5.0 -5.0 10.0) (struct :`Pitch` 48.0 :`Yaw` -160.0 :`Roll` -102.0))))
    (:`then_1`
      ;[1 1 1] Magnet Snap and Respawn
      (bind _outactors (`GameplayStatics.GetAllActorsOfClass` "/Game/Spawnable-ProduseCat_1/ProduseCat_1_BP.ProduseCat_1_BP_C")))
    (:`then_2`
      ;[1 1 1] Disables Hand Lines Collision with Large Display BP
      (bind _outactors_2 (`GameplayStatics.GetAllActorsOfClass` "/Game/VR_Table+Display/LargeDisplay_BP.LargeDisplay_BP_C")))
    (:`then_3`
      (`self.EnableInput` (`GameplayStatics.GetPlayerController` 0)))
    (:`then_4`
      ;[1 1 1] Set Color
      (bind _output_get (set `self.StructVariable-White` (`self.StructVariable-White`) :!label _label_9))
      (bind _returnvalue (`PrimitiveComponent.CreateDynamicMaterialInstance` (`self.Periuta_v2_BODY`) (break `/Game/ProduseCat_1/ElectricBrushesColor_Struct` _output_get) (`.BodyMaterialInstance_30_39E56B104B3FE8EE7B22DC84962C15C1` (break `/Game/ProduseCat_1/ElectricBrushesColor_Struct` _output_get)) "None"))
      (`MaterialInstanceDynamic.SetVectorParameterValue` _returnvalue (`.BodyParameterName_31_9E53DF694185C6CCF32F8D9AB0B5B4AD` (break `/Game/ProduseCat_1/ElectricBrushesColor_Struct` _output_get)) (`KismetMathLibrary.Conv_ColorToLinearColor` (`.BodyColor_8_65E980EE487C516F3F129F9AF12EB4A3` (break `/Game/ProduseCat_1/ElectricBrushesColor_Struct` _output_get))))
      (bind _returnvalue_2 (`PrimitiveComponent.CreateDynamicMaterialInstance` (`self.Periuta_v2_BODY`) (`.HeadIndex_33_BB231F9442374977CE1A7881706B0598` (break `/Game/ProduseCat_1/ElectricBrushesColor_Struct` _output_get)) (`.HeadMaterialInstance_36_4FB533EA42B8987B2F6F0F974D770DD4` (break `/Game/ProduseCat_1/ElectricBrushesColor_Struct` _output_get)) "None"))
      (`MaterialInstanceDynamic.SetVectorParameterValue` _returnvalue_2 (`.HeadParameterName_39_40D4799846097843E29B0296B96B86AD` (break `/Game/ProduseCat_1/ElectricBrushesColor_Struct` _output_get)) (`KismetMathLibrary.Conv_ColorToLinearColor` (`.HeadColor_42_07FEDE354978477499C1A7A465522D5B` (break `/Game/ProduseCat_1/ElectricBrushesColor_Struct` _output_get))))
      (bind _returnvalue_3 (`PrimitiveComponent.CreateDynamicMaterialInstance` (`self.Periuta_v2_HEAD`) (`.BrushesIndex_45_1837C78A464E5D51026B71AB953D73C2` (break `/Game/ProduseCat_1/ElectricBrushesColor_Struct` _output_get)) (`.BrushesMaterialInstance_48_BEA0391E4551A9463B8348B4C8ECD973` (break `/Game/ProduseCat_1/ElectricBrushesColor_Struct` _output_get)) "None"))
      (`MaterialInstanceDynamic.SetVectorParameterValue` _returnvalue_3 (`.BrushesParameterName_51_889C4F52401210539476AD84AF48940B` (break `/Game/ProduseCat_1/ElectricBrushesColor_Struct` _output_get)) (`KismetMathLibrary.Conv_ColorToLinearColor` (`.BrushesColor_54_7DD91FF949D8A4EF8075838A7D8D8772` (break `/Game/ProduseCat_1/ElectricBrushesColor_Struct` _output_get))))
      (bind _returnvalue_4 (`PrimitiveComponent.CreateDynamicMaterialInstance` (`self.Periuta_v2_HEAD`) (`.BrushesHeadIndex_57_E26A9CA34AE57749570D3783E3D082DB` (break `/Game/ProduseCat_1/ElectricBrushesColor_Struct` _output_get)) (`.BrushesHeadMaterialInstance_60_5618EC9C47445EA61F695FB54CFF5AEA` (break `/Game/ProduseCat_1/ElectricBrushesColor_Struct` _output_get)) "None"))
      (`MaterialInstanceDynamic.SetVectorParameterValue` _returnvalue_4 (`.BrushesHeadParameterName_63_7433266A40A0F1B9BE8A7B818BCC6F04` (break `/Game/ProduseCat_1/ElectricBrushesColor_Struct` _output_get)) (`KismetMathLibrary.Conv_ColorToLinearColor` (`.BrushesHeadColor_66_408735F145DDB964135281A373F86533` (break `/Game/ProduseCat_1/ElectricBrushesColor_Struct` _output_get))))
      (bind _returnvalue_5 (`PrimitiveComponent.CreateDynamicMaterialInstance` (`self.Periuta_v2_BODY`) (`.InelMareIndex_69_B0F2AC0C44A4187639F85E81406A0752` (break `/Game/ProduseCat_1/ElectricBrushesColor_Struct` _output_get)) (`.InelMareMaterialInstance_73_594E06FB4CD2E65F6DCEEE833A5F0386` (break `/Game/ProduseCat_1/ElectricBrushesColor_Struct` _output_get)) "None"))
      (`MaterialInstanceDynamic.SetVectorParameterValue` _returnvalue_5 (`.InelMareParameterName_76_8C84963A436C60D81C84C9BA712CFD5C` (break `/Game/ProduseCat_1/ElectricBrushesColor_Struct` _output_get)) (`KismetMathLibrary.Conv_ColorToLinearColor` (`.InelMareColor_79_0A6231A14865A1AF5A0EE59414E7EA5A` (break `/Game/ProduseCat_1/ElectricBrushesColor_Struct` _output_get))))
      (bind _returnvalue_6 (`PrimitiveComponent.CreateDynamicMaterialInstance` (`self.Periuta_v2_BODY`) (`.RingIndex_82_871ED50647FB77D07972958DCE24D1E7` (break `/Game/ProduseCat_1/ElectricBrushesColor_Struct` _output_get)) (`.RingMaterialInstance_85_1E9583D7491CFBA37DA0A7841B8487DE` (break `/Game/ProduseCat_1/ElectricBrushesColor_Struct` _output_get)) "None"))
      (`MaterialInstanceDynamic.SetVectorParameterValue` _returnvalue_6 (`.RingParameterName_88_AADF6CD34E47343234F9E4A537F868E0` (break `/Game/ProduseCat_1/ElectricBrushesColor_Struct` _output_get)) (`KismetMathLibrary.Conv_ColorToLinearColor` (`.RingColor_91_669D3370402E09A37916199ED6230F6C` (break `/Game/ProduseCat_1/ElectricBrushesColor_Struct` _output_get))))
      (set `self.StructVariable-LastColorChoosed` (`self.StructVariable-White`)))))

(event `InputAction|LeftHandXClick` :consume false
  (params (Key :type "Key Structure"))
  ;[1 1 1] Hand Controller X and A Clicked
  (:`Pressed`
    (set `self.LeftHandXClicked` true))
  (:`Released`
    (set `self.LeftHandXClicked` false)))

(event `InputAction|RightHandAClick` :consume false
  (params (Key :type "Key Structure"))
  ;[1 1 1] Hand Controller X and A Clicked
  (:`Pressed`
    (set `self.RightHandAClicked` true))
  (:`Released`
    (set `self.RightHandAClicked` false)))

(event `self.BoxCollisionPeriuta1_v2.OnComponentBeginOverlap`
  (params (OverlappedComponent :type "PrimitiveComponent Object Reference") (OtherActor :type "Actor Object Reference") (OtherComp :type "PrimitiveComponent Object Reference") (OtherBodyIndex :type Integer) (bFromSweep :type Boolean) (SweepResult :type "HitResult Structure (by ref)"))
  ;[1 1 1] Magnet Snap and Respawn
  (`/Engine/EditorBlueprintResources/StandardMacros.FlipFlop`
    (:`B`
      (`|ExecutionSequence`
        (:`then_0`
          (`self.K2_DestroyActor`)
          (`/Engine/EditorBlueprintResources/StandardMacros.DoOnce` false
            (:`Completed`
              (bind _periuta1_v2cubebase (`/Game/Spawnable-ProduseCat_1/ProduseCat_1_BP.Periuta1_v2CubeBase` (`|GetArrayItem` (stale `self.ReceiveBeginPlay` _outactors))))
              (bind (_returnvalue_x _returnvalue_y _returnvalue_z) (`KismetMathLibrary.BreakVector` (`SceneComponent.K2_GetComponentLocation` _periuta1_v2cubebase)))
              ;;[0.4932 0 1] REPLACE HERE
              (bind _returnvalue (`|SpawnActorFromClass` "Periuta1_v2_BP_C" (`KismetMathLibrary.MakeTransform` (`KismetMathLibrary.MakeVector` _returnvalue_x _returnvalue_y (+ _returnvalue_z 10.0)) (struct :`Yaw` 180.0) (4.0 4.0 4.0)) "AdjustIfPossibleButAlwaysSpawn" "OverrideRootScale" null null))
              ;[1 1 1] Remember Last Color
              (`|ExecutionSequence`
                (:`then_0`
                  (bind _output_get (set `self.StructVariable-LastColorChoosed` (`self.StructVariable-LastColorChoosed`)))
                  (bind _periuta_v2_body (`/Game/ProduseCat_1/Periuta1_v2_BP.Periuta_v2_BODY` _returnvalue))
                  (bind _returnvalue_2 (`PrimitiveComponent.CreateDynamicMaterialInstance` _periuta_v2_body (break `/Game/ProduseCat_1/ElectricBrushesColor_Struct` _output_get) (`.BodyMaterialInstance_30_39E56B104B3FE8EE7B22DC84962C15C1` (break `/Game/ProduseCat_1/ElectricBrushesColor_Struct` _output_get)) "None"))
                  (`MaterialInstanceDynamic.SetVectorParameterValue` _returnvalue_2 (`.BodyParameterName_31_9E53DF694185C6CCF32F8D9AB0B5B4AD` (break `/Game/ProduseCat_1/ElectricBrushesColor_Struct` _output_get)) (`KismetMathLibrary.Conv_ColorToLinearColor` (`.BodyColor_8_65E980EE487C516F3F129F9AF12EB4A3` (break `/Game/ProduseCat_1/ElectricBrushesColor_Struct` _output_get))))
                  (bind _returnvalue_3 (`PrimitiveComponent.CreateDynamicMaterialInstance` _periuta_v2_body (`.HeadIndex_33_BB231F9442374977CE1A7881706B0598` (break `/Game/ProduseCat_1/ElectricBrushesColor_Struct` _output_get)) (`.HeadMaterialInstance_36_4FB533EA42B8987B2F6F0F974D770DD4` (break `/Game/ProduseCat_1/ElectricBrushesColor_Struct` _output_get)) "None"))
                  (`MaterialInstanceDynamic.SetVectorParameterValue` _returnvalue_3 (`.HeadParameterName_39_40D4799846097843E29B0296B96B86AD` (break `/Game/ProduseCat_1/ElectricBrushesColor_Struct` _output_get)) (`KismetMathLibrary.Conv_ColorToLinearColor` (`.HeadColor_42_07FEDE354978477499C1A7A465522D5B` (break `/Game/ProduseCat_1/ElectricBrushesColor_Struct` _output_get))))
                  (bind _periuta_v2_head (`/Game/ProduseCat_1/Periuta1_v2_BP.Periuta_v2_HEAD` _returnvalue))
                  (bind _returnvalue_4 (`PrimitiveComponent.CreateDynamicMaterialInstance` _periuta_v2_head (`.BrushesIndex_45_1837C78A464E5D51026B71AB953D73C2` (break `/Game/ProduseCat_1/ElectricBrushesColor_Struct` _output_get)) (`.BrushesMaterialInstance_48_BEA0391E4551A9463B8348B4C8ECD973` (break `/Game/ProduseCat_1/ElectricBrushesColor_Struct` _output_get)) "None"))
                  (`MaterialInstanceDynamic.SetVectorParameterValue` _returnvalue_4 (`.BrushesParameterName_51_889C4F52401210539476AD84AF48940B` (break `/Game/ProduseCat_1/ElectricBrushesColor_Struct` _output_get)) (`KismetMathLibrary.Conv_ColorToLinearColor` (`.BrushesColor_54_7DD91FF949D8A4EF8075838A7D8D8772` (break `/Game/ProduseCat_1/ElectricBrushesColor_Struct` _output_get))))
                  (bind _returnvalue_5 (`PrimitiveComponent.CreateDynamicMaterialInstance` _periuta_v2_head (`.BrushesHeadIndex_57_E26A9CA34AE57749570D3783E3D082DB` (break `/Game/ProduseCat_1/ElectricBrushesColor_Struct` _output_get)) (`.BrushesHeadMaterialInstance_60_5618EC9C47445EA61F695FB54CFF5AEA` (break `/Game/ProduseCat_1/ElectricBrushesColor_Struct` _output_get)) "None"))
                  (`MaterialInstanceDynamic.SetVectorParameterValue` _returnvalue_5 (`.BrushesHeadParameterName_63_7433266A40A0F1B9BE8A7B818BCC6F04` (break `/Game/ProduseCat_1/ElectricBrushesColor_Struct` _output_get)) (`KismetMathLibrary.Conv_ColorToLinearColor` (`.BrushesHeadColor_66_408735F145DDB964135281A373F86533` (break `/Game/ProduseCat_1/ElectricBrushesColor_Struct` _output_get))))
                  (bind _returnvalue_6 (`PrimitiveComponent.CreateDynamicMaterialInstance` _periuta_v2_body (`.InelMareIndex_69_B0F2AC0C44A4187639F85E81406A0752` (break `/Game/ProduseCat_1/ElectricBrushesColor_Struct` _output_get)) (`.InelMareMaterialInstance_73_594E06FB4CD2E65F6DCEEE833A5F0386` (break `/Game/ProduseCat_1/ElectricBrushesColor_Struct` _output_get)) "None"))
                  (`MaterialInstanceDynamic.SetVectorParameterValue` _returnvalue_6 (`.InelMareParameterName_76_8C84963A436C60D81C84C9BA712CFD5C` (break `/Game/ProduseCat_1/ElectricBrushesColor_Struct` _output_get)) (`KismetMathLibrary.Conv_ColorToLinearColor` (`.InelMareColor_79_0A6231A14865A1AF5A0EE59414E7EA5A` (break `/Game/ProduseCat_1/ElectricBrushesColor_Struct` _output_get))))
                  (bind _returnvalue_7 (`PrimitiveComponent.CreateDynamicMaterialInstance` _periuta_v2_body (`.RingIndex_82_871ED50647FB77D07972958DCE24D1E7` (break `/Game/ProduseCat_1/ElectricBrushesColor_Struct` _output_get)) (`.RingMaterialInstance_85_1E9583D7491CFBA37DA0A7841B8487DE` (break `/Game/ProduseCat_1/ElectricBrushesColor_Struct` _output_get)) "None"))
                  (`MaterialInstanceDynamic.SetVectorParameterValue` _returnvalue_7 (`.RingParameterName_88_AADF6CD34E47343234F9E4A537F868E0` (break `/Game/ProduseCat_1/ElectricBrushesColor_Struct` _output_get)) (`KismetMathLibrary.Conv_ColorToLinearColor` (`.RingColor_91_669D3370402E09A37916199ED6230F6C` (break `/Game/ProduseCat_1/ElectricBrushesColor_Struct` _output_get)))))))))
        (:`then_1`
          ;;[1 1 1] If Brush Sound is Playing, on overlap, it plays the brush stop sound attached to CubeBase
          (if (`self.MySoundIsPlaying`)
            (`GameplayStatics.SpawnSoundAttached` "/Game/Audio/ElectricBrush/ElectricBrush_Stop_Cue.ElectricBrush_Stop_Cue" _periuta1_v2cubebase "None" (0.0 0.0 0.0) (struct) "SnapToTargetIncludingScale" false 1.0 1.0 0.0 null null false)))))))

(event `self.CubeNegru.OnComponentBeginOverlap`
  (params (OverlappedComponent :type "PrimitiveComponent Object Reference") (OtherActor :type "Actor Object Reference") (OtherComp :type "PrimitiveComponent Object Reference") (OtherBodyIndex :type Integer) (bFromSweep :type Boolean) (SweepResult :type "HitResult Structure (by ref)"))
  ;[1 1 1] Set Color
  (bind _output_get (set `self.StructVariable-Black` (`self.StructVariable-Black`)))
  (bind _returnvalue (`PrimitiveComponent.CreateDynamicMaterialInstance` (`self.Periuta_v2_BODY`) (break `/Game/ProduseCat_1/ElectricBrushesColor_Struct` _output_get) (`.BodyMaterialInstance_30_39E56B104B3FE8EE7B22DC84962C15C1` (break `/Game/ProduseCat_1/ElectricBrushesColor_Struct` _output_get)) "None"))
  (`MaterialInstanceDynamic.SetVectorParameterValue` _returnvalue (`.BodyParameterName_31_9E53DF694185C6CCF32F8D9AB0B5B4AD` (break `/Game/ProduseCat_1/ElectricBrushesColor_Struct` _output_get)) (`KismetMathLibrary.Conv_ColorToLinearColor` (`.BodyColor_8_65E980EE487C516F3F129F9AF12EB4A3` (break `/Game/ProduseCat_1/ElectricBrushesColor_Struct` _output_get))))
  (bind _returnvalue_2 (`PrimitiveComponent.CreateDynamicMaterialInstance` (`self.Periuta_v2_BODY`) (`.HeadIndex_33_BB231F9442374977CE1A7881706B0598` (break `/Game/ProduseCat_1/ElectricBrushesColor_Struct` _output_get)) (`.HeadMaterialInstance_36_4FB533EA42B8987B2F6F0F974D770DD4` (break `/Game/ProduseCat_1/ElectricBrushesColor_Struct` _output_get)) "None"))
  (`MaterialInstanceDynamic.SetVectorParameterValue` _returnvalue_2 (`.HeadParameterName_39_40D4799846097843E29B0296B96B86AD` (break `/Game/ProduseCat_1/ElectricBrushesColor_Struct` _output_get)) (`KismetMathLibrary.Conv_ColorToLinearColor` (`.HeadColor_42_07FEDE354978477499C1A7A465522D5B` (break `/Game/ProduseCat_1/ElectricBrushesColor_Struct` _output_get))))
  (bind _returnvalue_3 (`PrimitiveComponent.CreateDynamicMaterialInstance` (`self.Periuta_v2_HEAD`) (`.BrushesIndex_45_1837C78A464E5D51026B71AB953D73C2` (break `/Game/ProduseCat_1/ElectricBrushesColor_Struct` _output_get)) (`.BrushesMaterialInstance_48_BEA0391E4551A9463B8348B4C8ECD973` (break `/Game/ProduseCat_1/ElectricBrushesColor_Struct` _output_get)) "None"))
  (`MaterialInstanceDynamic.SetVectorParameterValue` _returnvalue_3 (`.BrushesParameterName_51_889C4F52401210539476AD84AF48940B` (break `/Game/ProduseCat_1/ElectricBrushesColor_Struct` _output_get)) (`KismetMathLibrary.Conv_ColorToLinearColor` (`.BrushesColor_54_7DD91FF949D8A4EF8075838A7D8D8772` (break `/Game/ProduseCat_1/ElectricBrushesColor_Struct` _output_get))))
  (bind _returnvalue_4 (`PrimitiveComponent.CreateDynamicMaterialInstance` (`self.Periuta_v2_HEAD`) (`.BrushesHeadIndex_57_E26A9CA34AE57749570D3783E3D082DB` (break `/Game/ProduseCat_1/ElectricBrushesColor_Struct` _output_get)) (`.BrushesHeadMaterialInstance_60_5618EC9C47445EA61F695FB54CFF5AEA` (break `/Game/ProduseCat_1/ElectricBrushesColor_Struct` _output_get)) "None"))
  (`MaterialInstanceDynamic.SetVectorParameterValue` _returnvalue_4 (`.BrushesHeadParameterName_63_7433266A40A0F1B9BE8A7B818BCC6F04` (break `/Game/ProduseCat_1/ElectricBrushesColor_Struct` _output_get)) (`KismetMathLibrary.Conv_ColorToLinearColor` (`.BrushesHeadColor_66_408735F145DDB964135281A373F86533` (break `/Game/ProduseCat_1/ElectricBrushesColor_Struct` _output_get))))
  (bind _returnvalue_5 (`PrimitiveComponent.CreateDynamicMaterialInstance` (`self.Periuta_v2_BODY`) (`.InelMareIndex_69_B0F2AC0C44A4187639F85E81406A0752` (break `/Game/ProduseCat_1/ElectricBrushesColor_Struct` _output_get)) (`.InelMareMaterialInstance_73_594E06FB4CD2E65F6DCEEE833A5F0386` (break `/Game/ProduseCat_1/ElectricBrushesColor_Struct` _output_get)) "None"))
  (`MaterialInstanceDynamic.SetVectorParameterValue` _returnvalue_5 (`.InelMareParameterName_76_8C84963A436C60D81C84C9BA712CFD5C` (break `/Game/ProduseCat_1/ElectricBrushesColor_Struct` _output_get)) (`KismetMathLibrary.Conv_ColorToLinearColor` (`.InelMareColor_79_0A6231A14865A1AF5A0EE59414E7EA5A` (break `/Game/ProduseCat_1/ElectricBrushesColor_Struct` _output_get))))
  (bind _returnvalue_6 (`PrimitiveComponent.CreateDynamicMaterialInstance` (`self.Periuta_v2_BODY`) (`.RingIndex_82_871ED50647FB77D07972958DCE24D1E7` (break `/Game/ProduseCat_1/ElectricBrushesColor_Struct` _output_get)) (`.RingMaterialInstance_85_1E9583D7491CFBA37DA0A7841B8487DE` (break `/Game/ProduseCat_1/ElectricBrushesColor_Struct` _output_get)) "None"))
  (`MaterialInstanceDynamic.SetVectorParameterValue` _returnvalue_6 (`.RingParameterName_88_AADF6CD34E47343234F9E4A537F868E0` (break `/Game/ProduseCat_1/ElectricBrushesColor_Struct` _output_get)) (`KismetMathLibrary.Conv_ColorToLinearColor` (`.RingColor_91_669D3370402E09A37916199ED6230F6C` (break `/Game/ProduseCat_1/ElectricBrushesColor_Struct` _output_get))))
  (set `self.StructVariable-LastColorChoosed` (`self.StructVariable-Black`)))

(event `self.CubeAlb.OnComponentBeginOverlap`
  (params (OverlappedComponent :type "PrimitiveComponent Object Reference") (OtherActor :type "Actor Object Reference") (OtherComp :type "PrimitiveComponent Object Reference") (OtherBodyIndex :type Integer) (bFromSweep :type Boolean) (SweepResult :type "HitResult Structure (by ref)"))
  ;[1 1 1] Set Color
  (goto _label_9))

(event `self.CubeRoz.OnComponentBeginOverlap`
  (params (OverlappedComponent :type "PrimitiveComponent Object Reference") (OtherActor :type "Actor Object Reference") (OtherComp :type "PrimitiveComponent Object Reference") (OtherBodyIndex :type Integer) (bFromSweep :type Boolean) (SweepResult :type "HitResult Structure (by ref)"))
  ;[1 1 1] Set Color
  (bind _output_get (set `self.StructVariable-Pink` (`self.StructVariable-Pink`)))
  (bind _returnvalue (`PrimitiveComponent.CreateDynamicMaterialInstance` (`self.Periuta_v2_BODY`) (break `/Game/ProduseCat_1/ElectricBrushesColor_Struct` _output_get) (`.BodyMaterialInstance_30_39E56B104B3FE8EE7B22DC84962C15C1` (break `/Game/ProduseCat_1/ElectricBrushesColor_Struct` _output_get)) "None"))
  (`MaterialInstanceDynamic.SetVectorParameterValue` _returnvalue (`.BodyParameterName_31_9E53DF694185C6CCF32F8D9AB0B5B4AD` (break `/Game/ProduseCat_1/ElectricBrushesColor_Struct` _output_get)) (`KismetMathLibrary.Conv_ColorToLinearColor` (`.BodyColor_8_65E980EE487C516F3F129F9AF12EB4A3` (break `/Game/ProduseCat_1/ElectricBrushesColor_Struct` _output_get))))
  (bind _returnvalue_2 (`PrimitiveComponent.CreateDynamicMaterialInstance` (`self.Periuta_v2_BODY`) (`.HeadIndex_33_BB231F9442374977CE1A7881706B0598` (break `/Game/ProduseCat_1/ElectricBrushesColor_Struct` _output_get)) (`.HeadMaterialInstance_36_4FB533EA42B8987B2F6F0F974D770DD4` (break `/Game/ProduseCat_1/ElectricBrushesColor_Struct` _output_get)) "None"))
  (`MaterialInstanceDynamic.SetVectorParameterValue` _returnvalue_2 (`.HeadParameterName_39_40D4799846097843E29B0296B96B86AD` (break `/Game/ProduseCat_1/ElectricBrushesColor_Struct` _output_get)) (`KismetMathLibrary.Conv_ColorToLinearColor` (`.HeadColor_42_07FEDE354978477499C1A7A465522D5B` (break `/Game/ProduseCat_1/ElectricBrushesColor_Struct` _output_get))))
  (bind _returnvalue_3 (`PrimitiveComponent.CreateDynamicMaterialInstance` (`self.Periuta_v2_HEAD`) (`.BrushesIndex_45_1837C78A464E5D51026B71AB953D73C2` (break `/Game/ProduseCat_1/ElectricBrushesColor_Struct` _output_get)) (`.BrushesMaterialInstance_48_BEA0391E4551A9463B8348B4C8ECD973` (break `/Game/ProduseCat_1/ElectricBrushesColor_Struct` _output_get)) "None"))
  (`MaterialInstanceDynamic.SetVectorParameterValue` _returnvalue_3 (`.BrushesParameterName_51_889C4F52401210539476AD84AF48940B` (break `/Game/ProduseCat_1/ElectricBrushesColor_Struct` _output_get)) (`KismetMathLibrary.Conv_ColorToLinearColor` (`.BrushesColor_54_7DD91FF949D8A4EF8075838A7D8D8772` (break `/Game/ProduseCat_1/ElectricBrushesColor_Struct` _output_get))))
  (bind _returnvalue_4 (`PrimitiveComponent.CreateDynamicMaterialInstance` (`self.Periuta_v2_HEAD`) (`.BrushesHeadIndex_57_E26A9CA34AE57749570D3783E3D082DB` (break `/Game/ProduseCat_1/ElectricBrushesColor_Struct` _output_get)) (`.BrushesHeadMaterialInstance_60_5618EC9C47445EA61F695FB54CFF5AEA` (break `/Game/ProduseCat_1/ElectricBrushesColor_Struct` _output_get)) "None"))
  (`MaterialInstanceDynamic.SetVectorParameterValue` _returnvalue_4 (`.BrushesHeadParameterName_63_7433266A40A0F1B9BE8A7B818BCC6F04` (break `/Game/ProduseCat_1/ElectricBrushesColor_Struct` _output_get)) (`KismetMathLibrary.Conv_ColorToLinearColor` (`.BrushesHeadColor_66_408735F145DDB964135281A373F86533` (break `/Game/ProduseCat_1/ElectricBrushesColor_Struct` _output_get))))
  (bind _returnvalue_5 (`PrimitiveComponent.CreateDynamicMaterialInstance` (`self.Periuta_v2_BODY`) (`.InelMareIndex_69_B0F2AC0C44A4187639F85E81406A0752` (break `/Game/ProduseCat_1/ElectricBrushesColor_Struct` _output_get)) (`.InelMareMaterialInstance_73_594E06FB4CD2E65F6DCEEE833A5F0386` (break `/Game/ProduseCat_1/ElectricBrushesColor_Struct` _output_get)) "None"))
  (`MaterialInstanceDynamic.SetVectorParameterValue` _returnvalue_5 (`.InelMareParameterName_76_8C84963A436C60D81C84C9BA712CFD5C` (break `/Game/ProduseCat_1/ElectricBrushesColor_Struct` _output_get)) (`KismetMathLibrary.Conv_ColorToLinearColor` (`.InelMareColor_79_0A6231A14865A1AF5A0EE59414E7EA5A` (break `/Game/ProduseCat_1/ElectricBrushesColor_Struct` _output_get))))
  (bind _returnvalue_6 (`PrimitiveComponent.CreateDynamicMaterialInstance` (`self.Periuta_v2_BODY`) (`.RingIndex_82_871ED50647FB77D07972958DCE24D1E7` (break `/Game/ProduseCat_1/ElectricBrushesColor_Struct` _output_get)) (`.RingMaterialInstance_85_1E9583D7491CFBA37DA0A7841B8487DE` (break `/Game/ProduseCat_1/ElectricBrushesColor_Struct` _output_get)) "None"))
  (`MaterialInstanceDynamic.SetVectorParameterValue` _returnvalue_6 (`.RingParameterName_88_AADF6CD34E47343234F9E4A537F868E0` (break `/Game/ProduseCat_1/ElectricBrushesColor_Struct` _output_get)) (`KismetMathLibrary.Conv_ColorToLinearColor` (`.RingColor_91_669D3370402E09A37916199ED6230F6C` (break `/Game/ProduseCat_1/ElectricBrushesColor_Struct` _output_get))))
  (set `self.StructVariable-LastColorChoosed` (`self.StructVariable-Pink`)))

(fn `UserConstructionScript`)