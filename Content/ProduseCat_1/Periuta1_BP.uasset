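; VR grabbable Dr. Mayer toothbrush (Periuta1) product with a selectable color and magnetic snap back to its display base.
; Tick drives haptics while grabbed with X or A held, and rolling the brush reveals pink, white and black overlap cubes.
; Cube overlaps recolor via dynamic materials, with body color set before the choice updates and neck after.
; Every second box overlap destroys and respawns the brush above ProduseCat_1_BP's base, reapplying the color.
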(event `self.ReceiveTick`
  (params (DeltaSeconds :type "Float (single-precision)"))
  (bind _returnvalue (`GameplayStatics.GetPlayerController` 0))
  (bind _cuberoz (`self.CubeRoz`))
  (bind _cubenegru (`self.CubeNegru`))
  (bind _cubealb (`self.CubeAlb`))
  (bind _returnvalue_roll (`KismetMathLibrary.BreakRotator` (`SceneComponent.K2_GetComponentRotation` (`self.Periuta_Dr_Mayer1`))))
  (bind _grabbed (`/UVRF/Hands/Grabable.IsGrabbed` (`self.Grabable`)))
  ;[1 0 0.8452] Event Tick
  (`|ExecutionSequence`
    (:`then_0`
      ;[1 1 1] Vibrate Controllers on grab and click
      (if (and _grabbed (`self.LeftHandXClicked`))
        (`PlayerController.PlayHapticEffect` _returnvalue "/Game/Playground/Objects/Bow/BowTreble.BowTreble" "Left" 4.0 true)
        (else
          (`PlayerController.StopHapticEffect` _returnvalue "Left"))))
    (:`then_1`
      (if (and _grabbed (`self.RightHandAClicked`))
        (`PlayerController.PlayHapticEffect` _returnvalue "/Game/Playground/Objects/Bow/BowTreble.BowTreble" "Right" 4.0 true)
        (else
          (`PlayerController.StopHapticEffect` _returnvalue "Right"))))
    (:`then_2`
      ;[1 1 1] Tilt to choose color
      (if (< _returnvalue_roll -30.0)
        (`SceneComponent.SetVisibility` _cuberoz true false)
        (`SceneComponent.SetVisibility` _cubealb true false)
        (`SceneComponent.SetVisibility` _cubenegru true false)
        (set `PrimitiveComponent.bGenerateOverlapEvents` true _cuberoz)
        (set `PrimitiveComponent.bGenerateOverlapEvents` true _cubenegru)
        (set `PrimitiveComponent.bGenerateOverlapEvents` true _cubealb)
        (else
          (`SceneComponent.SetVisibility` _cuberoz false false)
          (`SceneComponent.SetVisibility` _cubealb false false)
          (`SceneComponent.SetVisibility` _cubenegru false false)
          (set `PrimitiveComponent.bGenerateOverlapEvents` false _cuberoz)
          (set `PrimitiveComponent.bGenerateOverlapEvents` false _cubenegru)
          (set `PrimitiveComponent.bGenerateOverlapEvents` false _cubealb))))))

(event `InputAction|LeftHandXClick`
  (params (Key :type "Key Structure"))
  ;[1 1 1] Vibrate Controllers on grab and click
  (:`Pressed`
    (set `self.LeftHandXClicked` true))
  (:`Released`
    (set `self.LeftHandXClicked` false)))

(event `InputAction|RightHandAClick`
  (params (Key :type "Key Structure"))
  ;[1 1 1] Vibrate Controllers on grab and click
  (:`Pressed`
    (set `self.RightHandAClicked` true))
  (:`Released`
    (set `self.RightHandAClicked` false)))

(event `self.ReceiveBeginPlay`
  ;[0 1 0.001442] Begin Play
  (`|ExecutionSequence`
    (:`then_0`
      ;[1 1 1] Grabbed object position and rotation
      (`/UVRF/Hands/Grabable.SetFixedGrab` (`self.Grabable`) (`self.Periuta_Dr_Mayer1`) (`KismetMathLibrary.MakeTransform` (5.0 -5.0 10.0) (struct :`Pitch` -48.0 :`Yaw` 20.0 :`Roll` 102.0)) "/UVRF/Hands/Model/Animations/Grabs/grab_Periuta1.grab_Periuta1" (`KismetMathLibrary.MakeTransform` (5.0 -5.0 10.0) (struct :`Pitch` 48.0 :`Yaw` -160.0 :`Roll` -102.0))))
    (:`then_1`
      ;[1 1 1] Magnet Snap and Respawn
      (bind _outactors (`GameplayStatics.GetAllActorsOfClass` "/Game/Spawnable-ProduseCat_1/ProduseCat_1_BP.ProduseCat_1_BP_C")))))

(event `self.BoxCollisionPeriuta_Dr_Mayer1.OnComponentBeginOverlap`
  (params (OverlappedComponent :type "PrimitiveComponent Object Reference") (OtherActor :type "Actor Object Reference") (OtherComp :type "PrimitiveComponent Object Reference") (OtherBodyIndex :type Integer) (bFromSweep :type Boolean) (SweepResult :type "HitResult Structure (by ref)"))
  ;[1 1 1] Magnet Snap and Respawn
  (`/Engine/EditorBlueprintResources/StandardMacros.FlipFlop`
    (:`B`
      (`KismetSystemLibrary.PrintString` "Periuta1 Magnetic Snap")
      (`self.K2_DestroyActor`)
      (`/Engine/EditorBlueprintResources/StandardMacros.DoOnce` false
        (:`Completed`
          (bind (_returnvalue_x _returnvalue_y _returnvalue_z) (`KismetMathLibrary.BreakVector` (`SceneComponent.K2_GetComponentLocation` (`/Game/Spawnable-ProduseCat_1/ProduseCat_1_BP.Periuta1CubeBase` (`|GetArrayItem` (stale `self.ReceiveBeginPlay` _outactors))))))
          (bind _returnvalue (`|SpawnActorFromClass` "Periuta1_BP_C" (`KismetMathLibrary.MakeTransform` (`KismetMathLibrary.MakeVector` _returnvalue_x _returnvalue_y (+ _returnvalue_z 10.0)) (struct :`Yaw` 180.0) (4.0 4.0 4.0)) "AdjustIfPossibleButAlwaysSpawn" "OverrideRootScale" null null))
          (`|ExecutionSequence`
            (:`then_0`
              (bind _periuta_dr_mayer1 (`/Game/ProduseCat_1/Periuta1_BP.Periuta_Dr_Mayer1` _returnvalue))
              (bind _returnvalue_2 (`PrimitiveComponent.CreateDynamicMaterialInstance` _periuta_dr_mayer1 6 "/Game/ProduseCat_1/BodyColor_Inst.BodyColor_Inst" "None"))
              (`MaterialInstanceDynamic.SetVectorParameterValue` _returnvalue_2 "BodyColor" (`KismetMathLibrary.Conv_ColorToLinearColor` (`self.ChoosedBodyColor`))))
            (:`then_1`
              (bind _returnvalue_3 (`PrimitiveComponent.CreateDynamicMaterialInstance` _periuta_dr_mayer1 1 "/Game/ProduseCat_1/Gat_Inst.Gat_Inst" "None"))
              (`MaterialInstanceDynamic.SetVectorParameterValue` _returnvalue_3 "GatColor" (`KismetMathLibrary.Conv_ColorToLinearColor` (`self.ChoosedBodyColor`))))))))))

(event `self.CubeNegru.OnComponentBeginOverlap`
  (params (OverlappedComponent :type "PrimitiveComponent Object Reference") (OtherActor :type "Actor Object Reference") (OtherComp :type "PrimitiveComponent Object Reference") (OtherBodyIndex :type Integer) (bFromSweep :type Boolean) (SweepResult :type "HitResult Structure (by ref)"))
  (bind _periuta_dr_mayer1 (`self.Periuta_Dr_Mayer1`))
  ;[1 1 1] Set Color
  (`|ExecutionSequence`
    (:`then_0`
      (bind _returnvalue (`PrimitiveComponent.CreateDynamicMaterialInstance` _periuta_dr_mayer1 6 "/Game/ProduseCat_1/BodyColor_Inst.BodyColor_Inst" "None"))
      (`MaterialInstanceDynamic.SetVectorParameterValue` _returnvalue "BodyColor" (`KismetMathLibrary.Conv_ColorToLinearColor` (`self.ChoosedBodyColor`))))
    (:`then_1`
      (set `self.ChoosedBodyColor` (`self.Black`)))
    (:`then_2`
      (bind _returnvalue_2 (`PrimitiveComponent.CreateDynamicMaterialInstance` _periuta_dr_mayer1 1 "/Game/ProduseCat_1/Gat_Inst.Gat_Inst" "None"))
      (`MaterialInstanceDynamic.SetVectorParameterValue` _returnvalue_2 "GatColor" (`KismetMathLibrary.Conv_ColorToLinearColor` (`self.ChoosedBodyColor`))))))

(event `self.CubeAlb.OnComponentBeginOverlap`
  (params (OverlappedComponent :type "PrimitiveComponent Object Reference") (OtherActor :type "Actor Object Reference") (OtherComp :type "PrimitiveComponent Object Reference") (OtherBodyIndex :type Integer) (bFromSweep :type Boolean) (SweepResult :type "HitResult Structure (by ref)"))
  (bind _periuta_dr_mayer1 (`self.Periuta_Dr_Mayer1`))
  ;[1 1 1] Set Color
  (`|ExecutionSequence`
    (:`then_0`
      (bind _returnvalue (`PrimitiveComponent.CreateDynamicMaterialInstance` _periuta_dr_mayer1 6 "/Game/ProduseCat_1/BodyColor_Inst.BodyColor_Inst" "None"))
      (`MaterialInstanceDynamic.SetVectorParameterValue` _returnvalue "BodyColor" (`KismetMathLibrary.Conv_ColorToLinearColor` (`self.ChoosedBodyColor`))))
    (:`then_1`
      (set `self.ChoosedBodyColor` (`self.White`)))
    (:`then_2`
      (bind _returnvalue_2 (`PrimitiveComponent.CreateDynamicMaterialInstance` _periuta_dr_mayer1 1 "/Game/ProduseCat_1/Gat_Inst.Gat_Inst" "None"))
      (`MaterialInstanceDynamic.SetVectorParameterValue` _returnvalue_2 "GatColor" (`KismetMathLibrary.Conv_ColorToLinearColor` (`self.ChoosedBodyColor`))))))

(event `self.CubeRoz.OnComponentBeginOverlap`
  (params (OverlappedComponent :type "PrimitiveComponent Object Reference") (OtherActor :type "Actor Object Reference") (OtherComp :type "PrimitiveComponent Object Reference") (OtherBodyIndex :type Integer) (bFromSweep :type Boolean) (SweepResult :type "HitResult Structure (by ref)"))
  (bind _periuta_dr_mayer1 (`self.Periuta_Dr_Mayer1`))
  ;[1 1 1] Set Color
  (`|ExecutionSequence`
    (:`then_0`
      (bind _returnvalue (`PrimitiveComponent.CreateDynamicMaterialInstance` _periuta_dr_mayer1 6 "/Game/ProduseCat_1/BodyColor_Inst.BodyColor_Inst" "None"))
      (`MaterialInstanceDynamic.SetVectorParameterValue` _returnvalue "BodyColor" (`KismetMathLibrary.Conv_ColorToLinearColor` (`self.ChoosedBodyColor`))))
    (:`then_1`
      (set `self.ChoosedBodyColor` (`self.Pink`)))
    (:`then_2`
      (bind _returnvalue_2 (`PrimitiveComponent.CreateDynamicMaterialInstance` _periuta_dr_mayer1 1 "/Game/ProduseCat_1/Gat_Inst.Gat_Inst" "None"))
      (`MaterialInstanceDynamic.SetVectorParameterValue` _returnvalue_2 "GatColor" (`KismetMathLibrary.Conv_ColorToLinearColor` (`self.ChoosedBodyColor`))))))

(fn `UserConstructionScript`)