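; All_Data_Collector_BP links VR controller buttons to two grabbable Periuta brush actors, driving head rotation and haptics.
; Left X and right A input events set pressed flags.
; Each Tick it finds both brushes by class and, per hand, starts rotation and looping haptics if held and pressed, otherwise stopping both.
; Periuta2 is evaluated after Periuta1, so its stop calls can cancel haptics Periuta1 started on that hand.
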(event `InputAction|LeftHandXClick`
  (params (Key :type "Key Structure"))
  ;[1 1 1] Hand Controller X and A Clicked
  (:`Pressed`
    (set `self.LeftHandXClicked` true))
  (:`Released`
    (set `self.LeftHandXClicked` false)))

(event `InputAction|RightHandAClick`
  (params (Key :type "Key Structure"))
  ;[1 1 1] Hand Controller X and A Clicked
  (:`Pressed`
    (set `self.RightHandAClicked` true))
  (:`Released`
    (set `self.RightHandAClicked` false)))

(event `self.ReceiveTick`
  (params (DeltaSeconds :type "Float (single-precision)"))
  (bind _returnvalue (`GameplayStatics.GetPlayerController` 0))
  ;[1 0 0.7292] Tick
  (`|ExecutionSequence`
    (:`then_1`
      (bind _returnvalue_2 (`GameplayStatics.GetActorOfClass` "/Game/ProduseCat_1/Periuta1_v2_BP.Periuta1_v2_BP_C"))
      (bind _asperiuta_1_v_2_bp (cast `/Game/ProduseCat_1/Periuta1_v2_BP` _returnvalue_2))
      (`|ExecutionSequence`
        (:`then_0`
          (bind _grabbed (`/UVRF/Hands/Grabable.IsGrabbed` (`/Game/ProduseCat_1/Periuta1_v2_BP.Grabable` _asperiuta_1_v_2_bp)))
          (if (and _grabbed (`self.LeftHandXClicked`) (`/Game/ProduseCat_1/Periuta1_v2_BP.GrabbedByLeftHand` _asperiuta_1_v_2_bp))
            (`PlayerController.PlayHapticEffect` _returnvalue "/UVRF/Haptics/Periuta1.Periuta1" "Left" 4.0 true)
            (`/Game/ProduseCat_1/Periuta1_v2_BP.StartRotateHeadForLeftHandEvent` _asperiuta_1_v_2_bp)
            (else
              (`PlayerController.StopHapticEffect` _returnvalue "Left")
              (`/Game/ProduseCat_1/Periuta1_v2_BP.StopRotateHeadForLeftHandEvent` _asperiuta_1_v_2_bp))))
        (:`then_1`
          (if (and _grabbed (`self.RightHandAClicked`) (`/Game/ProduseCat_1/Periuta1_v2_BP.GrabbedByRightHand` _asperiuta_1_v_2_bp))
            (`PlayerController.PlayHapticEffect` _returnvalue "/UVRF/Haptics/Periuta1.Periuta1" "Right" 4.0 true)
            (`/Game/ProduseCat_1/Periuta1_v2_BP.StartRotateHeadForRightHandEvent` _asperiuta_1_v_2_bp)
            (else
              (`PlayerController.StopHapticEffect` _returnvalue "Right")
              (`/Game/ProduseCat_1/Periuta1_v2_BP.StopRotateHeadForRightHandEvent` _asperiuta_1_v_2_bp))))))
    (:`then_2`
      (bind _returnvalue_3 (`GameplayStatics.GetActorOfClass` "/Game/ProduseCat_1/Periuta2_v2_BP.Periuta2_v2_BP_C"))
      (bind _asperiuta_2_v_2_bp (cast `/Game/ProduseCat_1/Periuta2_v2_BP` _returnvalue_3))
      (`|ExecutionSequence`
        (:`then_0`
          (bind _grabbed_2 (`/UVRF/Hands/Grabable.IsGrabbed` (`/Game/ProduseCat_1/Periuta2_v2_BP.Grabable` _asperiuta_2_v_2_bp)))
          (if (and _grabbed_2 (`self.LeftHandXClicked`) (`/Game/ProduseCat_1/Periuta2_v2_BP.GrabbedByLeftHand` _asperiuta_2_v_2_bp))
            (`PlayerController.PlayHapticEffect` _returnvalue "/UVRF/Haptics/Periuta1.Periuta1" "Left" 4.0 true)
            (`/Game/ProduseCat_1/Periuta2_v2_BP.StartRotateHeadForLeftHandEvent` _asperiuta_2_v_2_bp)
            (else
              (`PlayerController.StopHapticEffect` _returnvalue "Left")
              (`/Game/ProduseCat_1/Periuta2_v2_BP.StopRotateHeadForLeftHandEvent` _asperiuta_2_v_2_bp))))
        (:`then_1`
          (if (and _grabbed_2 (`self.RightHandAClicked`) (`/Game/ProduseCat_1/Periuta2_v2_BP.GrabbedByRightHand` _asperiuta_2_v_2_bp))
            (`PlayerController.PlayHapticEffect` _returnvalue "/UVRF/Haptics/Periuta1.Periuta1" "Right" 4.0 true)
            (`/Game/ProduseCat_1/Periuta2_v2_BP.StartRotateHeadForRightHandEvent` _asperiuta_2_v_2_bp)
            (else
              (`PlayerController.StopHapticEffect` _returnvalue "Right")
              (`/Game/ProduseCat_1/Periuta2_v2_BP.StopRotateHeadForRightHandEvent` _asperiuta_2_v_2_bp))))))))

(fn `UserConstructionScript`)