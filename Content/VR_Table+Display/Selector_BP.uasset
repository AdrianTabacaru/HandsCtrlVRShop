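; Selector_BP is a VR selector button that reacts when something overlaps its collision box.
; Begin overlap plays a haptic pulse on the left or right controller, chosen by matching the overlapping component's display name to the VR pawn's line cylinders.
; It also plays the ZoomInOut timeline, which scales the button through additive local transforms.
; End overlap reverses the timeline from its end.
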(event `self.CollisionBox.OnComponentBeginOverlap`
  (params (OverlappedComponent :type "PrimitiveComponent Object Reference") (OtherActor :type "Actor Object Reference") (OtherComp :type "PrimitiveComponent Object Reference") (OtherBodyIndex :type Integer) (bFromSweep :type Boolean) (SweepResult :type "HitResult Structure (by ref)"))
  (bind _returnvalue (`GameplayStatics.GetPlayerController` 0))
  ;[1 1 1] Zoom In/Out
  ;[1 1 1] Vibrate Controller
  (`|ExecutionSequence`
    (:`then_0`
      (switch `name` (`KismetStringLibrary.Conv_StringToName` (`KismetSystemLibrary.GetDisplayName` OtherComp))
        (:`VRPawn_5.LeftLine Cylinder`
          (`PlayerController.PlayHapticEffect` _returnvalue "/UVRF/Haptics/Grab.Grab" "Left" 4.0 false))
        (:`VRPawn_5.RightLine Cylinder`
          (`PlayerController.PlayHapticEffect` _returnvalue "/UVRF/Haptics/Grab.Grab" "Right" 4.0 false))))
    (:`then_1`
      (bind (_direction _scaler) (`Timeline|ZoomIn-Out` :!via `PlayFromStart` :!label _label)
        (:`Update`
          (`SceneComponent.K2_AddLocalTransform` (`self.SelectButton`) (`KismetMathLibrary.MakeTransform` (0.0 0.0 0.0) (struct) _scaler) false false))))))

(event `self.CollisionBox.OnComponentEndOverlap`
  (params (OverlappedComponent :type "PrimitiveComponent Object Reference") (OtherActor :type "Actor Object Reference") (OtherComp :type "PrimitiveComponent Object Reference") (OtherBodyIndex :type Integer))
  ;[1 1 1] Zoom In/Out
  (goto _label :!via `ReverseFromEnd`))

(fn `UserConstructionScript`)