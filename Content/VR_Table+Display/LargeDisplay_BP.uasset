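; Large VR display actor that reveals a hand's pointer line while it overlaps the display and rotates with the right thumbstick.
; Begin/end overlap toggles the first VRPawn's left or right line, matched by display names hard-coded to the "VR Pawn 5" instance.
; Tick disables the other line's collision when one is visible, intending one-hand selection.
; The thumbstick axis value is added to the display's world yaw.
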(event `self.LargeDisplay.OnComponentBeginOverlap`
  (params (OverlappedComponent :type "PrimitiveComponent Object Reference") (OtherActor :type "Actor Object Reference") (OtherComp :type "PrimitiveComponent Object Reference") (OtherBodyIndex :type Integer) (bFromSweep :type Boolean) (SweepResult :type "HitResult Structure (by ref)"))
  ;[1 1 1] Make Hand Lines Visible/Invisible
  (switch `name` (`KismetStringLibrary.Conv_StringToName` (`KismetSystemLibrary.GetDisplayName` OtherComp))
    (:`VRPawn_5.LeftLine Cylinder`
      (bind _output (`|GetArrayItem` (stale `self.ReceiveBeginPlay` _outactors)))
      (`SceneComponent.SetVisibility` (`/UVRF/Pawn/VRPawn.LeftLine` _output) true false))
    (:`VRPawn_5.RightLine Cylinder`
      (`SceneComponent.SetVisibility` (`/UVRF/Pawn/VRPawn.RightLine` _output) true false))))

(event `InputAxis|RightMotionControllerThumbstick`
  (params (AxisValue :type "Float (single-precision)"))
  (bind _largedisplay (`self.LargeDisplay`))
  (bind (_returnvalue_roll _returnvalue_pitch _returnvalue_yaw) (`KismetMathLibrary.BreakRotator` (`SceneComponent.GetSocketRotation` _largedisplay "None")))
  ;[1 1 1] Display Rotation using Right Thumb XY
  (`SceneComponent.K2_SetWorldRotation` _largedisplay (`KismetMathLibrary.MakeRotator` 0.0 0.0 (+ AxisValue _returnvalue_yaw)) false false))

(event `self.ReceiveBeginPlay`
  ;[0 1 0.2463] Begin Play
  (`|ExecutionSequence`
    (:`then_0`
      ;[1 1 1] Make Hand Lines Visible/Invisible
      (bind _outactors (`GameplayStatics.GetAllActorsOfClass` "/UVRF/Pawn/VRPawn.VRPawn_C")))))

(event `self.ReceiveTick`
  (params (DeltaSeconds :type "Float (single-precision)"))
  ;[1 0 0.9036] Event Tick
  (`|ExecutionSequence`
    (:`then_0`
      (bind _output (`|GetArrayItem` (stale `self.ReceiveBeginPlay` _outactors)))
      (bind _leftline (`/UVRF/Pawn/VRPawn.LeftLine` _output))
      ;[1 1 1] Use only one hand at a time for selection
      (if (`SceneComponent.IsVisible` _leftline)
        (bind _rightline (`/UVRF/Pawn/VRPawn.RightLine` _output))
        (`PrimitiveComponent.SetCollisionEnabled` _rightline "NoCollision")
        (`PrimitiveComponent.SetCollisionEnabled` _leftline "QueryAndPhysics")
        (else
          (`PrimitiveComponent.SetCollisionEnabled` _rightline "QueryAndPhysics"))))
    (:`then_1`
      (if (`SceneComponent.IsVisible` _rightline)
        (`PrimitiveComponent.SetCollisionEnabled` _leftline "NoCollision")
        (`PrimitiveComponent.SetCollisionEnabled` _rightline "QueryAndPhysics")
        (else
          (`PrimitiveComponent.SetCollisionEnabled` _leftline "QueryAndPhysics"))))))

(event `self.LargeDisplay.OnComponentEndOverlap`
  (params (OverlappedComponent :type "PrimitiveComponent Object Reference") (OtherActor :type "Actor Object Reference") (OtherComp :type "PrimitiveComponent Object Reference") (OtherBodyIndex :type Integer))
  ;[1 1 1] Make Hand Lines Visible/Invisible
  (switch `name` (`KismetStringLibrary.Conv_StringToName` (`KismetSystemLibrary.GetDisplayName` OtherComp))
    (:`VRPawn_5.LeftLine Cylinder`
      (bind _output (`|GetArrayItem` (stale `self.ReceiveBeginPlay` _outactors)))
      (`SceneComponent.SetVisibility` (`/UVRF/Pawn/VRPawn.LeftLine` _output) false false))
    (:`VRPawn_5.RightLine Cylinder`
      (`SceneComponent.SetVisibility` (`/UVRF/Pawn/VRPawn.RightLine` _output) false false))))

(fn `UserConstructionScript`)